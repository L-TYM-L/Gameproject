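; First-person multiplayer player character that maps movement, look and fire input.
; On possession, the authority creates an auto rifle through BPWeaponManager and selects it.
; Fire input is routed to a server event that uses the manager's current weapon.
; GetVisibleMesh returns the hands mesh for the locally controlled player and the body mesh for everyone else.
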(event `self.ReceivePossessed`
  (params (NewController :type "Controller Object Reference"))
  (`/Engine/EditorBlueprintResources/ActorMacros.Switch Has Authority`
    (:`Authority`
      (bind _weapon (`/Game/Blueprints/Components/Player/BP_WeaponManager.CreateWeapon` (`self.BP_WeaponManager`) "/Game/Blueprints/Weapons/BP_Weapon_AutoRifles.BP_Weapon_AutoRifles_C"))
      (`/Game/Blueprints/Components/Player/BP_WeaponManager.SelectWeapon` (`self.BP_WeaponManager`) _weapon))))

(event `InputAction|Fire`
  (params (Key :type "Key Structure" :default "AnyKey"))
  (:`Pressed`
    (`self.Server_Fire`)))

(event `InputAxis|LookUp`
  (params (AxisValue :type "Float (single-precision)"))
  (`self.AddControllerPitchInput` AxisValue))

(event `Server_Fire`
  (`/Game/Blueprints/Weapons/BP_WEapon.UseWeapon` (`/Game/Blueprints/Components/Player/BP_WeaponManager.CurrentWeapon` (`self.BP_WeaponManager`))))

(event `InputAxis|MoveForward`
  (params (AxisValue :type "Float (single-precision)"))
  (`self.AddMovementInput` (`self.GetActorForwardVector`) AxisValue))

(event `InputAxis|Turn`
  (params (AxisValue :type "Float (single-precision)"))
  (`self.AddControllerYawInput` AxisValue))

(event `InputAxis|MoveRight`
  (params (AxisValue :type "Float (single-precision)"))
  (`self.AddMovementInput` (`self.GetActorRightVector`) AxisValue))

(fn `GetVisibleMesh`
  (returns (SkeletalMesh :type "SkeletalMeshComponent Object Reference"))
  (return (select `bool` (`self.IsLocallyControlled`) :`false` (`self.Mesh`) :`true` (`self.HandsMesh`))))

(fn `UserConstructionScript`)